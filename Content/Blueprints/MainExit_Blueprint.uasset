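; Level exit that sends an overlapping Creature to a random unvisited room, or to Boss_Room once three rooms have been picked.
; BeginPlay restores the room counter and six visited flags from the RoomTick save slot.
; On overlap it rerolls until it hits an unused room, saves the flags and incremented counter, and opens that level.
; Opening the boss level also deletes the save slot, resetting the run.
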(event EventBeginPlay
  (bind _returnvalue (SaveGame|DoesSaveGameExist "RoomTick"))
  (if _returnvalue
    (bind _returnvalue_2 (SaveGame|LoadGamefromSlot "RoomTick"))
    (bind _asroom_tick_save (Utilities|Casting|CastToRoomTickSave _returnvalue_2))
    (Variables|Default|SetBossTick (Variables|/Game/Blueprints/Saves/RoomTickSave.RoomTickSave_C|GetBossTickSave _asroom_tick_save))
    (bind _asroom_tick_save_2 (Utilities|Casting|CastToRoomTickSave _returnvalue_2))
    (Variables|Default|SetRoom1Get (Variables|/Game/Blueprints/Saves/RoomTickSave.RoomTickSave_C|GetRoom1Save _asroom_tick_save_2))
    (bind _asroom_tick_save_3 (Utilities|Casting|CastToRoomTickSave _returnvalue_2))
    (Variables|Default|SetRoom2Get (Variables|/Game/Blueprints/Saves/RoomTickSave.RoomTickSave_C|GetRoom2Save _asroom_tick_save_3))
    (bind _asroom_tick_save_4 (Utilities|Casting|CastToRoomTickSave _returnvalue_2))
    (Variables|Default|SetRoom3Get (Variables|/Game/Blueprints/Saves/RoomTickSave.RoomTickSave_C|GetRoom3Save _asroom_tick_save_4))
    (bind _asroom_tick_save_5 (Utilities|Casting|CastToRoomTickSave _returnvalue_2))
    (Variables|Default|SetRoom4Get (Variables|/Game/Blueprints/Saves/RoomTickSave.RoomTickSave_C|GetRoom4Save _asroom_tick_save_5))
    (bind _asroom_tick_save_6 (Utilities|Casting|CastToRoomTickSave _returnvalue_2))
    (Variables|Default|SetRoom5Get (Variables|/Game/Blueprints/Saves/RoomTickSave.RoomTickSave_C|GetRoom5Save _asroom_tick_save_6))
    (bind _asroom_tick_save_7 (Utilities|Casting|CastToRoomTickSave _returnvalue_2))
    (Variables|Default|SetRoom6Get (Variables|/Game/Blueprints/Saves/RoomTickSave.RoomTickSave_C|GetRoom6Save _asroom_tick_save_7))))

(event Collision|EventActorBeginOverlap
  (params (OtherActor :type Actor%20Object%20Reference))
  (Utilities|Casting|CastToCreature OtherActor)
  (if (> (Variables|Default|GetBossTick) 2)
    (Game|OpenLevel(byName) "Boss_Room")
    (SaveGame|DeleteGameinSlot "RoomTick")
    (else
      (bind _returnvalue (SaveGame|CreateSaveGameObject "/Game/Blueprints/Saves/RoomTickSave.RoomTickSave_C"))
      (bind _output_get (Variables|Default|SetRandom2 (Math|Random|RandomInteger 6) :!label _label))
      (bind _output_get_2 (Variables|Default|SetSave_Ref _returnvalue))
      (Variables|/Game/Blueprints/Saves/RoomTickSave.RoomTickSave_C|SetRoom1Save _returnvalue (Variables|Default|GetRoom1Get))
      (SaveGame|SaveGametoSlot _output_get_2 "RoomTick")
      (bind _output_get_3 (Variables|Default|SetSave_Ref _returnvalue))
      (Variables|/Game/Blueprints/Saves/RoomTickSave.RoomTickSave_C|SetRoom2Save _returnvalue (Variables|Default|GetRoom2Get))
      (SaveGame|SaveGametoSlot _output_get_3 "RoomTick")
      (bind _output_get_4 (Variables|Default|SetSave_Ref _returnvalue))
      (Variables|/Game/Blueprints/Saves/RoomTickSave.RoomTickSave_C|SetRoom3Save _returnvalue (Variables|Default|GetRoom3Get))
      (SaveGame|SaveGametoSlot _output_get_4 "RoomTick")
      (bind _output_get_5 (Variables|Default|SetSave_Ref _returnvalue))
      (Variables|/Game/Blueprints/Saves/RoomTickSave.RoomTickSave_C|SetRoom4Save _returnvalue (Variables|Default|GetRoom4Get))
      (SaveGame|SaveGametoSlot _output_get_5 "RoomTick")
      (bind _output_get_6 (Variables|Default|SetSave_Ref _returnvalue))
      (Variables|/Game/Blueprints/Saves/RoomTickSave.RoomTickSave_C|SetRoom5Save _returnvalue (Variables|Default|GetRoom5Get))
      (SaveGame|SaveGametoSlot _output_get_6 "RoomTick")
      (bind _output_get_7 (Variables|Default|SetSave_Ref _returnvalue))
      (Variables|/Game/Blueprints/Saves/RoomTickSave.RoomTickSave_C|SetRoom6Save _returnvalue (Variables|Default|GetRoom6Get))
      (SaveGame|SaveGametoSlot _output_get_7 "RoomTick")
      (switch int _output_get
        (:0
          (if (Variables|Default|GetRoom1Get)
            (goto _label)
            (else
              (Variables|Default|SetRoom1Get true)
              (bind _output_get_8 (Variables|Default|SetSave_Ref _returnvalue))
              (Variables|/Game/Blueprints/Saves/RoomTickSave.RoomTickSave_C|SetRoom1Save _returnvalue (Variables|Default|GetRoom1Get))
              (SaveGame|SaveGametoSlot _output_get_8 "RoomTick")
              (Game|OpenLevel(byName) "Room1"))))
        (:1
          (if (Variables|Default|GetRoom2Get)
            (goto _label)
            (else
              (Variables|Default|SetRoom2Get true)
              (bind _output_get_9 (Variables|Default|SetSave_Ref _returnvalue))
              (Variables|/Game/Blueprints/Saves/RoomTickSave.RoomTickSave_C|SetRoom2Save _returnvalue (Variables|Default|GetRoom2Get))
              (SaveGame|SaveGametoSlot _output_get_9 "RoomTick")
              (Game|OpenLevel(byName) "Room2"))))
        (:2
          (if (Variables|Default|GetRoom3Get)
            (goto _label)
            (else
              (Variables|Default|SetRoom3Get true)
              (bind _output_get_10 (Variables|Default|SetSave_Ref _returnvalue))
              (Variables|/Game/Blueprints/Saves/RoomTickSave.RoomTickSave_C|SetRoom3Save _returnvalue (Variables|Default|GetRoom3Get))
              (SaveGame|SaveGametoSlot _output_get_10 "RoomTick")
              (Game|OpenLevel(byName) "Room3"))))
        (:3
          (if (Variables|Default|GetRoom4Get)
            (goto _label)
            (else
              (Variables|Default|SetRoom4Get true)
              (bind _output_get_11 (Variables|Default|SetSave_Ref _returnvalue))
              (Variables|/Game/Blueprints/Saves/RoomTickSave.RoomTickSave_C|SetRoom4Save _returnvalue (Variables|Default|GetRoom4Get))
              (SaveGame|SaveGametoSlot _output_get_11 "RoomTick")
              (Game|OpenLevel(byName) "Room4"))))
        (:4
          (if (Variables|Default|GetRoom5Get)
            (goto _label)
            (else
              (Variables|Default|SetRoom5Get true)
              (bind _output_get_12 (Variables|Default|SetSave_Ref _returnvalue))
              (Variables|/Game/Blueprints/Saves/RoomTickSave.RoomTickSave_C|SetRoom5Save _returnvalue (Variables|Default|GetRoom5Get))
              (SaveGame|SaveGametoSlot _output_get_12 "RoomTick")
              (Game|OpenLevel(byName) "Room5"))))
        (:5
          (if (Variables|Default|GetRoom6Get)
            (goto _label)
            (else
              (Variables|Default|SetRoom6Get true)
              (bind _output_get_13 (Variables|Default|SetSave_Ref _returnvalue))
              (Variables|/Game/Blueprints/Saves/RoomTickSave.RoomTickSave_C|SetRoom6Save _returnvalue (Variables|Default|GetRoom6Get))
              (SaveGame|SaveGametoSlot _output_get_13 "RoomTick")
              (Game|OpenLevel(byName) "Room6")))))
      (Math|Integer|IncrementInt (Variables|Default|GetBossTick)
        (:%20%20
          (bind _output_get_14 (Variables|Default|SetSave_Ref _returnvalue))
          (Variables|/Game/Blueprints/Saves/RoomTickSave.RoomTickSave_C|SetBossTickSave _returnvalue (Variables|Default|GetBossTick))
          (SaveGame|SaveGametoSlot _output_get_14 "RoomTick"))))))

(event EventTick
  (params (DeltaSeconds :type Float%20%28single-precision%29)))

(fn ConstructionScript)