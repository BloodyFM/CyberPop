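; Player character Blueprint handling hit feedback, cursor aiming, pausing and death.
; OnHit briefly scales both meshes and flashes a red outline through dynamic materials on NewMesh, which follows Mesh via master pose.
; Tick deletes the RoomTick save and shows game over at zero Hp, and orbits AimProjectile toward the cursor.
; Right mouse shows that indicator when attack and DashCharge allow, then turns the actor on release; debug key 3 wipes the save.
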(event EventBeginPlay
  (Class|SkinnedMeshComponent|SetMasterPoseComponent (Variables|Default|Getnewmesh) (Variables|Character|GetMesh) false))

(event Collision|EventActorBeginOverlap
  (params (OtherActor :type Actor%20Object%20Reference)))

(event EventOnHit
  (Variables|Default|Setshake 0.1)
  (for _index (range 0 5)
    (bind _returnvalue (Rendering|Material|CreateDynamicMaterialInstance (Variables|Default|GetNewMesh) _index "/Game/CartoonCelShader/Materials/CelShader/Mob_instances/character_outl.character_outl" "None" :!class /Script/Engine.PrimitiveComponent))
    (Rendering|Material|SetVectorParameterValue _returnvalue "Outline Color" "(R=100.000000,G=0.000000,B=0.000000,A=1.000000)" :!class /Script/Engine.MaterialInstanceDynamic)
    (Rendering|Material|SetScalarParameterValue _returnvalue "Outline Emissive Intensity" 1e+02 :!class /Script/Engine.MaterialInstanceDynamic))
  (Utilities|FlowControl|Sequence
    (:then_0
      (Transformation|SetRelativeScale3D (Variables|Character|GetMesh) "1.150000,1.150000,1.150000")
      (Transformation|SetRelativeScale3D (Variables|Default|GetNewMesh) "1.150000,1.150000,1.150000")
      (Utilities|FlowControl|Delay 0.1)
      (Transformation|SetRelativeScale3D (Variables|Character|GetMesh) "1.000000,1.000000,1.000000")
      (Transformation|SetRelativeScale3D (Variables|Default|GetNewMesh) "1.000000,1.000000,1.000000")
      (Utilities|FlowControl|Delay 0.1)
      (for _index_2 (range 0 5)
        (bind _returnvalue_2 (Rendering|Material|CreateDynamicMaterialInstance (Variables|Default|GetNewMesh) _index_2 "/Game/CartoonCelShader/Materials/CelShader/Mob_instances/character_outl.character_outl" "None" :!class /Script/Engine.PrimitiveComponent))
        (Rendering|Material|SetVectorParameterValue _returnvalue_2 "Outline Color" "(R=0.000000,G=0.000000,B=0.000000,A=1.000000)" :!class /Script/Engine.MaterialInstanceDynamic)
        (Rendering|Material|SetScalarParameterValue _returnvalue_2 "Outline Emissive Intensity" 1.0 :!class /Script/Engine.MaterialInstanceDynamic)))))

(event EventTick
  (params (DeltaSeconds :type Float%20%28single-precision%29))
  (bind _returnvalue (Game|GetPlayerController 0))
  (bind _returnvalue_2 (Transformation|GetActorLocation))
  (bind _returnvalue_3 (Game|GetPlayerController 0))
  (bind _hitresult (Game|Player|GetHitResultUnderCursorbyChannel _returnvalue_3 "TraceTypeQuery1" true))
  (bind _location (Collision|BreakHitResult _hitresult))
  (bind _returnvalue_4 (- _location _returnvalue_2))
  (bind _returnvalue_5 (Math|Vector|Normalize _returnvalue_4))
  (Utilities|FlowControl|Sequence
    (:then_0
      (if (<= (Variables|Default|Gethp) 0.0)
        (SaveGame|DeleteGameinSlot "RoomTick")
        (bind _returnvalue_6 (UserInterface|CreateWidget "/Game/Menus/GameOverScreenWidget.GameOverScreenWidget_C" _returnvalue))
        (UserInterface|Viewport|AddtoViewport _returnvalue_6 0)
        (Variables|/Script/Engine.PlayerController|SetbShowMouseCursor _returnvalue true)))
    (:then_1
      (if (> (Variables|Default|Getshake) 0.0)
        (bind _output_get (Variables|Default|Setshake (- (Variables|Default|Getshake) 1.0)))))
    (:then_2
      (Transformation|SetWorldLocationAndRotation (Variables|Default|GetAimProjectile) (+ _returnvalue_2 (* _returnvalue_5 2e+02)) (Math|Rotator|MakeRotator 0.0 9e+01 (+ (.yaw (Math|Rotator|FindLookatRotation (Variables|Default|GetStart) _returnvalue_5)) 9e+01)) false false))))

(event Input|KeyboardEvents|3
  (params (Key :type Key%20Structure :default "None"))
  (:Pressed
    (SaveGame|DeleteGameinSlot "RoomTick")
    (Development|PrintString "Deleted game")))

(event Input|MouseEvents|RightMouseButton
  (params (Key :type Key%20Structure :default "None"))
  (bind _aimprojectile (Variables|Default|GetAimProjectile))
  (:Pressed
    (if (Variables|Default|GetbCanAttack)
      (if (>= (Variables|Default|GetDashCharge) 3e+01)
        (Rendering|SetVisibility _aimprojectile true true)
        (Variables|Default|SetTooEarly false)
        (else
          (Variables|Default|SetTooEarly true :!label _label)))
      (else
        (goto _label))))
  (:Released
    (if (not (Variables|Default|GetTooEarly))
      (Rendering|SetVisibility _aimprojectile false true)
      (Transformation|SetActorRotation (Math|Rotator|MakeRotator 0.0 0.0 (.yaw (Math|Rotator|FindLookatRotation (Variables|Default|GetStart) (Math|Vector|Normalize (- (.Location (Collision|BreakHitResult (.HitResult (Game|Player|GetHitResultUnderCursorbyChannel (Game|GetPlayerController 0) "TraceTypeQuery1" true)))) (Transformation|GetActorLocation))))))))))

(event Input|KeyboardEvents|P
  (params (Key :type Key%20Structure :default "None"))
  (bind _returnvalue (Game|GetPlayerController 0))
  (:Pressed
    (bind _returnvalue_2 (UserInterface|CreateWidget "/Game/Menus/PauseMenu_Widget.PauseMenu_Widget_C" (Game|GetPlayerController 0)))
    (bind _output_get (Variables|Default|SetPause%20Menu _returnvalue_2))
    (UserInterface|Viewport|AddtoViewport _output_get 10)
    (Variables|/Script/Engine.PlayerController|SetbShowMouseCursor _returnvalue true)
    (Input|SetInputModeUIOnly _returnvalue _output_get "DoNotLock")
    (Game|SetGamePaused true)))

(fn ConstructionScript)