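; GameMode Blueprint that assigns the player to one of two placed characters, Main1_BP or Main2_BP, based on the class stored in the game instance.
; On BeginPlay it copies PlayerClass from GameInstance_BP into DefaultPawnClass and compares it to Main1_BP.
; It then possesses the matching level actor with the first player controller and destroys the other one.
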(event EventBeginPlay
  (bind _asgame_instance_bp (Utilities|Casting|CastToGameInstance_BP (Game|GetGameInstance)))
  (bind _output_get (Variables|Default|SetDefaultPawnClass (Variables|/Game/Blueprints/GameInstance_BP.GameInstance_BP_C|GetPlayerClass _asgame_instance_bp)))
  (if (== _output_get "/Game/Blueprints/Main1_BP.Main1_BP_C")
    (bind _returnvalue (Actor|GetActorOfClass "/Game/Blueprints/Main1_BP.Main1_BP_C"))
    (Pawn|Possess (Game|GetPlayerController 0) _returnvalue)
    (bind _returnvalue_2 (Actor|GetActorOfClass "/Game/Blueprints/Main2_BP.Main2_BP_C"))
    (Actor|DestroyActor _returnvalue_2)
    (else
      (bind _returnvalue_3 (Actor|GetActorOfClass "/Game/Blueprints/Main2_BP.Main2_BP_C"))
      (Pawn|Possess (Game|GetPlayerController 0) _returnvalue_3)
      (bind _returnvalue_4 (Actor|GetActorOfClass "/Game/Blueprints/Main1_BP.Main1_BP_C"))
      (Actor|DestroyActor _returnvalue_4))))

(event EventTick
  (params (DeltaSeconds :type Float%20%28single-precision%29)))

(fn ConstructionScript)