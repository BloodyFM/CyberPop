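; Teleporter actor with a trigger Box and a Spawn box that relocates Creatures entering the trigger.
; On Box overlap it casts the other actor to Creature, prints a debug "Hello", and proceeds only if the overlapping component is that creature's first capsule component.
; The creature then teleports, without sweep, to a random point inside the Spawn box's bounds.
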(event OnComponentBeginOverlap(Box)
  (params (OverlappedComponent :type Primitive%20Component%20Object%20Reference) (OtherActor :type Actor%20Object%20Reference) (OtherComp :type Primitive%20Component%20Object%20Reference) (OtherBodyIndex :type Integer) (bFromSweep :type Boolean) (SweepResult :type Hit%20Result%20Structure%20%28by%20ref%29))
  (bind _spawn (Variables|Default|Getspawn))
  (bind _ascreature (Utilities|Casting|CastToCreature OtherActor))
  (Development|PrintString "Hello")
  (if (== OtherComp (Utilities|Array|Get(acopy) (Actor|GetComponentsByClass _ascreature "/Script/Engine.CapsuleComponent")))
    (Transformation|SetActorLocation _ascreature (Math|Random|RandomPointinBoundingBox (Transformation|GetWorldLocation _spawn) (Variables|/Script/Engine.BoxComponent|GetBoxExtent _spawn)) false true)))

(event EventBeginPlay)

(event Collision|EventActorBeginOverlap
  (params (OtherActor :type Actor%20Object%20Reference)))

(event EventTick
  (params (DeltaSeconds :type Float%20%28single-precision%29)))

(fn ConstructionScript)