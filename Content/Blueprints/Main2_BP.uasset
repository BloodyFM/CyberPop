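; Player Blueprint that handles pausing, death and a visible shield.
; On BeginPlay it hides the shield mesh and slaves NewMesh to the main mesh's pose; shield events toggle visibility, with the off event also calling DeactivateShield.
; P opens a pause widget with UI-only input and pauses the game.
; Tick polls Hp and, every frame it is depleted, deletes the RoomTick save and creates a Game Over widget with the cursor shown.
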(event EventBeginPlay
  (Class|SkinnedMeshComponent|SetMasterPoseComponent (Variables|Default|GetNewMesh) (Variables|Character|GetMesh) false)
  (Rendering|SetVisibility (Variables|Default|GetShieldMesh) false false))

(event Collision|EventActorBeginOverlap
  (params (OtherActor :type Actor%20Object%20Reference)))

(event EventTick
  (params (DeltaSeconds :type Float%20%28single-precision%29))
  (bind _returnvalue (Game|GetPlayerController 0))
  (if (<= (Variables|Default|Gethp) 0.0)
    (SaveGame|DeleteGameinSlot "RoomTick")
    (bind _returnvalue_2 (UserInterface|CreateWidget "/Game/Menus/GameOverScreenWidget.GameOverScreenWidget_C" _returnvalue))
    (UserInterface|Viewport|AddtoViewport _returnvalue_2 0)
    (Variables|/Script/Engine.PlayerController|SetbShowMouseCursor _returnvalue true)))

(event EventShieldOpacityon
  (Rendering|SetVisibility (Variables|Default|GetShieldMesh) true false))

(event EventShieldOpacityOff
  (Rendering|SetVisibility (Variables|Default|GetShieldMesh) false false)
  (Class|Main2|DeactivateShield))

(event Input|KeyboardEvents|P
  (params (Key :type Key%20Structure :default "None"))
  (bind _returnvalue (Game|GetPlayerController 0))
  (:Pressed
    (bind _returnvalue_2 (UserInterface|CreateWidget "/Game/Menus/PauseMenu_Widget.PauseMenu_Widget_C" (Game|GetPlayerController 0)))
    (bind _output_get (Variables|Default|SetPause%20Menu _returnvalue_2))
    (UserInterface|Viewport|AddtoViewport _output_get 10)
    (Variables|/Script/Engine.PlayerController|SetbShowMouseCursor _returnvalue true)
    (Input|SetInputModeUIOnly _returnvalue 0 "DoNotLock")
    (Game|SetGamePaused true)))

(fn ConstructionScript)