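; BossFightManager_BP is an actor that picks and spawns the boss for a fight based on the player's class.
; On BeginPlay it reads PlayerClass from GameInstance_BP, spawning Boss2Class for Main1_BP and Boss1Class for any other class.
; The boss spawns at the manager's own transform and is stored in the Boss variable.
; A leftover "Hello" debug print runs first, and nothing spawns if the game instance cast fails.
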(event EventBeginPlay
  (bind _asgame_instance_bp (Utilities|Casting|CastToGameInstance_BP (Game|GetGameInstance)))
  (Development|PrintString "Hello")
  (if (== (Variables|/Game/Blueprints/GameInstance_BP.GameInstance_BP_C|GetPlayerClass _asgame_instance_bp) "/Game/Blueprints/Main1_BP.Main1_BP_C")
    (bind _returnvalue (Game|SpawnActorfromClass (Variables|Default|GetBoss2Class) (Transformation|GetActorTransform) "Undefined" 0 0))
    (Variables|Default|SetBoss _returnvalue)
    (else
      (bind _returnvalue_2 (Game|SpawnActorfromClass (Variables|Default|GetBoss1Class) (Transformation|GetActorTransform) "Undefined" 0 0))
      (Variables|Default|SetBoss _returnvalue_2))))

(event Collision|EventActorBeginOverlap
  (params (OtherActor :type Actor%20Object%20Reference)))

(event EventTick
  (params (DeltaSeconds :type Float%20%28single-precision%29)))

(fn ConstructionScript)