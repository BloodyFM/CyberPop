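; Grunt enemy Blueprint that gives visual hit feedback on a two-mesh body, with NewMesh following Mesh's pose as master component.
; OnHit briefly enlarges both meshes and flashes a red emissive outline through a dynamic Drone_outl material instance, then restores scale and darkens the outline.
; Tick counts down a Shake timer set on hit, but the sine-based vertical offset meant to use it is disconnected.
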(event EventBeginPlay
  (Class|SkinnedMeshComponent|SetMasterPoseComponent (Variables|Default|GetNewMesh) (Variables|Character|GetMesh) false))

(event Collision|EventActorBeginOverlap
  (params (OtherActor :type Actor%20Object%20Reference)))

(event EventTick
  (params (DeltaSeconds :type Float%20%28single-precision%29))
  (if (> (Variables|Default|Getshake) 0.0)
    (bind _output_get (Variables|Default|Setshake (- (Variables|Default|Getshake) DeltaSeconds)))))

(event EventOnHit
  (Variables|Default|Setshake 0.1)
  (bind _returnvalue (Rendering|Material|CreateDynamicMaterialInstance (Variables|Default|GetNewMesh) 0 "/Game/CartoonCelShader/Materials/Outline/drone_outl.drone_outl" "None" :!class /Script/Engine.PrimitiveComponent))
  (Rendering|Material|SetVectorParameterValue _returnvalue "Outline Color" "(R=100.000000,G=0.000000,B=0.000000,A=1.000000)" :!class /Script/Engine.MaterialInstanceDynamic)
  (Rendering|Material|SetScalarParameterValue _returnvalue "Outline Emissive Intensity" 1e+02 :!class /Script/Engine.MaterialInstanceDynamic)
  (Utilities|FlowControl|Sequence
    (:then_0
      (Transformation|SetRelativeScale3D (Variables|Character|GetMesh) "0.200000,0.200000,0.200000")
      (Transformation|SetRelativeScale3D (Variables|Default|GetNewMesh) "0.200000,0.200000,0.200000")
      (Utilities|FlowControl|Delay 0.1)
      (Transformation|SetRelativeScale3D (Variables|Character|GetMesh) "0.150000,0.150000,0.150000")
      (Transformation|SetRelativeScale3D (Variables|Default|GetNewMesh) "0.150000,0.150000,0.150000")
      (Utilities|FlowControl|Delay 0.1)
      (Rendering|Material|SetVectorParameterValue _returnvalue "Outline Color" "(R=0.000000,G=0.000000,B=0.000000,A=1.000000)" :!class /Script/Engine.MaterialInstanceDynamic)
      (Rendering|Material|SetScalarParameterValue _returnvalue "Outline Emissive Intensity" 1.0 :!class /Script/Engine.MaterialInstanceDynamic))))

(fn ConstructionScript)