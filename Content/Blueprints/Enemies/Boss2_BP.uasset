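; Boss 2 enemy character with a spline-guided jump attack and bullet spread attacks.
; Jumpattack builds a three-point arc to the target, optionally bending the landing vertical and showing an impact decal, then jumps and sets velocity toward the spline when its timeline finishes.
; ShootPattern alternates two two-handed spreads, while SplitFire fires mirrored pairs angled by remaining shots.
; Both firing modes draw down a shot counter that ResetFire refills.
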(event Custom|Jump%20attack
  (bind _returnvalue (Transformation|GetActorLocation))
  (Class|Boss2|InitiateJumptoCombatTarget)
  (CallFunction|CalculateJump)
  (Utilities|FlowControl|Sequence
    (:then_0
      (Character|Jump))
    (:then_1
      (bind _jumpcurve (Timeline|Jump_TL PlayFromStart)
        (:Finished
          (bind _output_get (Variables|/Script/Engine.MovementComponent|SetVelocity (Variables|Character|GetCharacterMovement) (* (Math|Vector|GetUnitDirection(Vector) _returnvalue (Spline|GetLocationatTime (Variables|Default|GetJumpSpline) _jumpcurve "World" false)) (* (Math|Vector|Distance(Vector) _returnvalue (Spline|GetLocationatTime (Variables|Default|GetJumpSpline) _jumpcurve "World" false)) 5e+01))))
          (Pawn|Input|AddMovementInput _output_get 1.0 false)
          (Rendering|SetVisibility (Variables|Default|GetImpactDecal) false true))))))

(event EventBeginPlay)

(event Collision|EventActorBeginOverlap
  (params (OtherActor :type Actor%20Object%20Reference)))

(event EventTick
  (params (DeltaSeconds :type Float%20%28single-precision%29)))

(fn ConstructionScript)

(fn ShowImpactMarker
  (Transformation|SetWorldLocation (Variables|Default|GetImpactDecal) (Variables|Default|GetJumpTargetLocation) false false)
  (Rendering|SetVisibility (Variables|Default|GetJumpSpline) true true))

(fn CalculateJump
  (bind _jumpstartlocation (Variables|Default|GetJumpStartLocation))
  (bind _jumptargetlocation (Variables|Default|GetJumpTargetLocation))
  (Spline|SetSplinePoints (Variables|Default|GetJumpSpline) (Utilities|Array|MakeArray _jumpstartlocation (* (+ _jumpstartlocation _jumptargetlocation) 0.5) _jumptargetlocation) "World" true)
  (if (Variables|Default|GetisLandingVertical)
    (Spline|SetTangentatSplinePoint (Variables|Default|GetJumpSpline) 2 (* "0, 0,-1.000000" (Math|Float|Clamp(Float) (Variables|Default|GetJumpDistance) 0.0 2e+03)) "World" true) ; optional, controlled by isLandingVertical\n\nT: 2nd point's tangent affected by distance of the jump \nF: basic arc with automatic tangents
    (CallFunction|ShowImpactMarker)))

(fn SplitFire
  (bind _returnvalue (Transformation|GetActorTransform))
  (bind _returnvalue_2 (Transformation|GetActorTransform))
  (Development|PrintString (Utilities|String|ToString(Float) (Variables|Default|GetShots)))
  (Game|SpawnActorfromClass (Variables|Default|GetBulletClass) (Math|Transform|MakeTransform (+ (.location _returnvalue) (* (Math|Vector|RotateVector (Transformation|GetActorForwardVector) (Math|Rotator|MakeRotator 0.0 0.0 (* (/ (Variables|Default|GetShots) (Variables|Default|GetMaxShots)) 65.0))) 5e+01)) (Math|Rotator|MakeRotator (.roll (.rotation _returnvalue)) (.pitch (.rotation _returnvalue)) (+ (.yaw (.rotation _returnvalue)) (* (/ (Variables|Default|GetShots) (Variables|Default|GetMaxShots)) 65.0))) "1,1,1") "AlwaysSpawn" 0 0)
  (Game|SpawnActorfromClass (Variables|Default|GetBulletClass) (Math|Transform|MakeTransform (+ (.location _returnvalue_2) (* (Math|Vector|RotateVector (Transformation|GetActorForwardVector) (Math|Rotator|MakeRotator 0.0 0.0 (* (/ (Variables|Default|GetShots) (Variables|Default|GetMaxShots)) -65.0))) 5e+01)) (Math|Rotator|MakeRotator (.roll (.rotation _returnvalue_2)) (.pitch (.rotation _returnvalue_2)) (+ (.yaw (.rotation _returnvalue_2)) (* (/ (Variables|Default|GetShots) (Variables|Default|GetMaxShots)) -65.0))) "1,1,1") "AlwaysSpawn" 0 0)
  (Variables|Default|SetShots (- (Variables|Default|GetShots) 1.0)))

(fn ResetFire
  (Variables|Default|SetShots (Variables|Default|GetMaxShots)))

(fn HideImpactMarker
  (Rendering|SetVisibility (Variables|Default|GetJumpSpline) false true))

(fn ShootPattern
  (bind _returnvalue (CallFunction|GetLocationinFront))
  ;[1 1 1] So it can be expanded if I have time
  (switch int (Variables|Default|GetPatternIndex)
    (:0
      (CallFunction|Pattern0 _returnvalue)
      (Variables|Default|SetPatternIndex 1))
    (:1
      (CallFunction|Pattern1 _returnvalue)
      (Variables|Default|SetPatternIndex 0))))

(fn GetLocationinFront
  (return (+ (Transformation|GetActorLocation) (* (Transformation|GetActorForwardVector) 5e+01))))

(fn Pattern0
  (params (SpawnLocation :type Vector))
  (bind _returnvalue (Transformation|GetActorRotation))
  (bind _returnvalue_2 (Transformation|GetActorRotation))
  (bind _returnvalue_3 (Transformation|GetActorForwardVector))
  (bind _returnvalue_4 (Transformation|GetActorForwardVector))
  (bind _bulletclass (Variables|Default|GetBulletClass))
  (bind _bulletclass_2 (Variables|Default|GetBulletClass))
  (bind _returnvalue_5 (Math|Vector|RotateVector _returnvalue_3 "0,90.000000, 0"))
  (bind _returnvalue_6 (Math|Vector|RotateVector _returnvalue_4 "0,90.000000, 0"))
  (bind _returnvalue_7 (+ (.yaw _returnvalue_2) -7.5))
  (bind _returnvalue_8 (+ (.yaw _returnvalue) 7.5))
  (bind _returnvalue_9 (* _returnvalue_5 3e+01))
  (bind _returnvalue_10 (* _returnvalue_6 -3e+01))
  (bind _returnvalue_11 (+ SpawnLocation _returnvalue_10))
  (bind _returnvalue_12 (+ SpawnLocation _returnvalue_9))
  ;[1 1 1] right hand
  (Game|SpawnActorfromClass _bulletclass_2 (Math|Transform|MakeTransform _returnvalue_12 (Math|Rotator|MakeRotator (.roll _returnvalue) (.pitch _returnvalue) _returnvalue_8) "1,1,1") "AlwaysSpawn" 0 0)
  (Game|SpawnActorfromClass _bulletclass_2 (Math|Transform|MakeTransform _returnvalue_12 (Math|Rotator|MakeRotator (.roll _returnvalue) (.pitch _returnvalue) (+ _returnvalue_8 15.0)) "1,1,1") "AlwaysSpawn" 0 0)
  ;[1 1 1] left hand
  (Game|SpawnActorfromClass _bulletclass (Math|Transform|MakeTransform _returnvalue_11 (Math|Rotator|MakeRotator (.roll _returnvalue_2) (.pitch _returnvalue_2) _returnvalue_7) "1,1,1") "AlwaysSpawn" 0 0)
  (Game|SpawnActorfromClass _bulletclass (Math|Transform|MakeTransform _returnvalue_11 (Math|Rotator|MakeRotator (.roll _returnvalue_2) (.pitch _returnvalue_2) (+ _returnvalue_7 -15.0)) "1,1,1") "AlwaysSpawn" 0 0)
  (Variables|Default|SetShots (- (Variables|Default|GetShots) 4.0)))

(fn Pattern1
  (params (SpawnLocation :type Vector))
  (bind _returnvalue (Transformation|GetActorRotation))
  (bind _returnvalue_2 (Transformation|GetActorRotation))
  (bind _returnvalue_3 (Transformation|GetActorForwardVector))
  (bind _returnvalue_4 (Transformation|GetActorForwardVector))
  (bind _bulletclass (Variables|Default|GetBulletClass))
  (bind _bulletclass_2 (Variables|Default|GetBulletClass))
  (bind _returnvalue_5 (Math|Vector|RotateVector _returnvalue_3 "0,90.000000, 0"))
  (bind _returnvalue_6 (Math|Vector|RotateVector _returnvalue_4 "0,90.000000, 0"))
  (bind _returnvalue_7 (+ (.yaw _returnvalue_2) -15.0))
  (bind _returnvalue_8 (+ (.yaw _returnvalue) 15.0))
  (bind _returnvalue_9 (* _returnvalue_5 3e+01))
  (bind _returnvalue_10 (* _returnvalue_6 -3e+01))
  (bind _returnvalue_11 (+ "0, 0, 0" _returnvalue_10))
  (bind _returnvalue_12 (+ SpawnLocation _returnvalue_9))
  ;[1 1 1] right hand
  (Game|SpawnActorfromClass _bulletclass_2 (Math|Transform|MakeTransform _returnvalue_12 (Math|Rotator|MakeRotator (.roll _returnvalue) (.pitch _returnvalue) (.yaw _returnvalue)) "1,1,1") "AlwaysSpawn" 0 0)
  (Game|SpawnActorfromClass _bulletclass_2 (Math|Transform|MakeTransform _returnvalue_12 (Math|Rotator|MakeRotator (.roll _returnvalue) (.pitch _returnvalue) _returnvalue_8) "1,1,1") "AlwaysSpawn" 0 0)
  (Game|SpawnActorfromClass _bulletclass_2 (Math|Transform|MakeTransform _returnvalue_12 (Math|Rotator|MakeRotator (.roll _returnvalue) (.pitch _returnvalue) (+ _returnvalue_8 15.0)) "1,1,1") "AlwaysSpawn" 0 0)
  ;[1 1 1] left hand
  (Game|SpawnActorfromClass _bulletclass (Math|Transform|MakeTransform _returnvalue_11 (Math|Rotator|MakeRotator (.roll _returnvalue_2) (.pitch _returnvalue_2) (.yaw _returnvalue_2)) "1,1,1") "AlwaysSpawn" 0 0)
  (Game|SpawnActorfromClass _bulletclass (Math|Transform|MakeTransform _returnvalue_11 (Math|Rotator|MakeRotator (.roll _returnvalue_2) (.pitch _returnvalue_2) _returnvalue_7) "1,1,1") "AlwaysSpawn" 0 0)
  (Game|SpawnActorfromClass _bulletclass (Math|Transform|MakeTransform _returnvalue_11 (Math|Rotator|MakeRotator (.roll _returnvalue_2) (.pitch _returnvalue_2) (+ _returnvalue_7 -15.0)) "1,1,1") "AlwaysSpawn" 0 0)
  (Variables|Default|SetShots (- (Variables|Default|GetShots) 6.0)))